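; spyObstacle is a patrolling hazard actor that moves back and forth and damages the BallPawn on hit.
; Tick offsets it along a normalized Direction without sweeping, while a looping timer reverses that direction every TimeToChange seconds.
; DiffGI from GI_HammyAdventure scales speed and sets the health lost per hit.
; A hit clears the pawn's CanDamage for a second but never checks that flag before subtracting health.
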(event Custom|ChangeDirection
  (Variables|Default|Setdirection (* (Variables|Default|Getdirection) -1.0)))

(event Collision|EventHit
  (params (MyComp :type Primitive%20Component%20Object%20Reference) (Other :type Actor%20Object%20Reference) (OtherComp :type Primitive%20Component%20Object%20Reference) (bSelfMoved :type Boolean) (HitLocation :type Vector :default "0, 0, 0") (HitNormal :type Vector :default "0, 0, 0") (NormalImpulse :type Vector :default "0, 0, 0") (Hit :type Hit%20Result%20Structure%20%28by%20ref%29))
  (bind _asball_pawn (Utilities|Casting|CastToBallPawn Other))
  (Variables|/Game/Blueprints/BallPawn.BallPawn_C|SetCanDamage _asball_pawn false)
  (Variables|/Game/Blueprints/BallPawn.BallPawn_C|SetPlayerHealth _asball_pawn (- (Variables|/Game/Blueprints/BallPawn.BallPawn_C|GetPlayerHealth _asball_pawn) (Variables|/Game/Blueprints/GI_HammyAdventure.GI_HammyAdventure_C|GetDiffGI (stale EventBeginPlay _asgi_hammy_adventure))))
  (Utilities|FlowControl|Delay 1.0)
  (Variables|/Game/Blueprints/BallPawn.BallPawn_C|SetCanDamage _asball_pawn true))

(event Collision|EventActorBeginOverlap
  (params (OtherActor :type Actor%20Object%20Reference)))

(event EventTick
  (params (DeltaSeconds :type Float%20%28single-precision%29))
  (Transformation|AddActorWorldOffset (* (Math|Vector|Normalize (Variables|Default|GetDirection)) (* (Variables|Default|GetSpeed) (Utilities|Time|GetWorldDeltaSeconds)))))

(event EventBeginPlay
  (bind _asgi_hammy_adventure (Utilities|Casting|CastToGI_HammyAdventure (Game|GetGameInstance)))
  (Variables|Default|Setspeed (* (Variables|Default|Getspeed) (Variables|/Game/Blueprints/GI_HammyAdventure.GI_HammyAdventure_C|GetDiffGI _asgi_hammy_adventure)))
  (Utilities|Time|SetTimerbyEvent (delegate Custom|ChangeDirection) (Variables|Default|GetTime%20to%20change) true))

(fn ConstructionScript)