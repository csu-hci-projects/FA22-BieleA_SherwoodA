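; Rainbow obstacle actor that moves back and forth along a configurable direction.
; Each Tick it offsets itself along the normalized Direction, scaled by Speed and delta time, without sweeping for collision.
; On BeginPlay a looping timer fires ChangeDirection every TimeToChange seconds, negating Direction to reverse the motion.
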(event Custom|ChangeDirection
  (Variables|Default|Setdirection (* (Variables|Default|Getdirection) -1.0)))

(event Collision|EventActorBeginOverlap
  (params (OtherActor :type Actor%20Object%20Reference)))

(event EventTick
  (params (DeltaSeconds :type Float%20%28single-precision%29))
  (Transformation|AddActorWorldOffset (* (Math|Vector|Normalize (Variables|Default|GetDirection)) (* (Variables|Default|GetSpeed) (Utilities|Time|GetWorldDeltaSeconds)))))

(event EventBeginPlay
  (Utilities|Time|SetTimerbyEvent (delegate Custom|ChangeDirection) (Variables|Default|GetTime%20to%20change) true))

(fn ConstructionScript)