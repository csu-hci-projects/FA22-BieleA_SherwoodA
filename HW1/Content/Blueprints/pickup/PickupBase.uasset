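; PickupBase is a score pickup actor that awards its Points to a BallPawn overlapping its Sphere.
; BeginPlay hides the PickupWidget and passes Points to its PickupText widget as the displayed value.
; On overlap it increments the pawn's score, plays a sound, spawns particles and shows the widget.
; The debug print, text animation and delayed destroy are unconnected, so the pickup stays in the level.
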(event OnComponentBeginOverlap(Sphere)
  (params (OverlappedComponent :type Primitive%20Component%20Object%20Reference) (OtherActor :type Actor%20Object%20Reference) (OtherComp :type Primitive%20Component%20Object%20Reference) (OtherBodyIndex :type Integer) (bFromSweep :type Boolean) (SweepResult :type Hit%20Result%20Structure%20%28by%20ref%29))
  ;[1 1 1] Increment Score
  (bind _asball_pawn (Utilities|Casting|CastToBallPawn OtherActor))
  (Default|IncrementScore _asball_pawn (Variables|Default|Getpoints))
  ;[1 1 1] Play Sound
  (Audio|PlaySound2D (Variables|Default|GetpickupSound) 1.0 1.0 0.0 0 0)
  ;[1 1 1] Emitter
  (Effects|SpawnEmitteratLocation (Variables|Default|GetpickupParticles) (Transformation|GetActorLocation))
  ;[1 1 1] Visibilty (Widget and Mesh)
  (Rendering|SetVisibility (Variables|Default|GetPickupWidget) true false))

(event Collision|EventActorBeginOverlap
  (params (OtherActor :type Actor%20Object%20Reference)))

(event EventTick
  (params (DeltaSeconds :type Float%20%28single-precision%29)))

(event EventBeginPlay
  (bind _pickupwidget (Variables|Default|GetPickupWidget))
  (Rendering|SetVisibility _pickupwidget false false)
  (bind _aspickup_text (Utilities|Casting|CastToPickupText (UserInterface|GetUserWidgetObject _pickupwidget)))
  (Variables|/Game/Blueprints/pickup/PickupText.PickupText_C|SetScoreValue _aspickup_text (Variables|Default|Getpoints)))

(fn ConstructionScript)